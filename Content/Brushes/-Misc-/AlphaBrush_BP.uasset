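; Landmass landscape brush that stamps an alpha heightmap texture, with falloff, blend mode and shaping controls, into the landscape's heightmap or weightmap.
; Initialize finds or spawns a shared LandmassBrushManager and requests a landscape update.
; Render feeds the incoming landscape render target, brush settings and actor transform into dynamic materials, then draws one into the manager's matching render target and returns it.
; Separate helpers export the distance field cache and force a jump flood.
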(event `self.Initialize`
  (params (InLandscapeTransform :type "Transform Structure (by ref)") (InLandscapeSize :type "IntPoint Structure (by ref)") (InLandscapeRenderTargetSize :type "IntPoint Structure (by ref)"))
  (`KismetSystemLibrary.PrintString` "Brush Initialize")
  (`self.Spawn or Update Manager` InLandscapeSize InLandscapeRenderTargetSize InLandscapeTransform)
  (`self.RequestLandscapeUpdate`))

(fn `Brush Setup`
  (params (`Landscape RT` :type "TextureRenderTarget2D Object Reference"))
  (`/Engine/EditorBlueprintResources/StandardMacros.IsValid` (`self.BrushManager`)
    (:`Is Valid`
      _)
    (:`Is Not Valid`
      _))
  (`self.Spawn or Update Manager` (`self.LS Size`) (`self.RT Res`) (`self.LSTransform`))
  (`/Landmass/Landscape/BlueprintBrushes/LandmassBrushManager.Set MPC Params` (`self.BrushManager`))
  (`self.Create MID if Needed` (`self.DrawBrushMID`) (`self.Brush Material`)
    (:`out`
      (`self.Create MID if Needed` (`self.WeightmapMID`) "/Landmass/Landscape/BlueprintBrushes/Materials/WaterPlugin/MeshBrush_Weightmap.MeshBrush_Weightmap"
        (:`out`
          (`MaterialInstanceDynamic.SetTextureParameterValue` (`self.DrawBrushMID`) "HeightRT" `Landscape RT`)
          (`MaterialInstanceDynamic.SetTextureParameterValue` (`self.WeightmapMID`) "HeightRT" `Landscape RT`)
          (`self.Set MID Params`))))))

(fn `Draw Brush Material`
  (bind _heightmap_rt (`/Landmass/Landscape/BlueprintBrushes/LandmassBrushManager.Heightmap RT` (`self.BrushManager`)))
  (bind _weightmap_rt (`/Landmass/Landscape/BlueprintBrushes/LandmassBrushManager.Weightmap RT` (`self.BrushManager`)))
  (if (`self.HeightmapRender`)
    (`KismetRenderingLibrary.ClearRenderTarget2D` _heightmap_rt)
    (`KismetRenderingLibrary.DrawMaterialToRenderTarget` _heightmap_rt (`self.DrawBrushMID`))
    (else
      (`KismetRenderingLibrary.ClearRenderTarget2D` _weightmap_rt)
      (`KismetRenderingLibrary.DrawMaterialToRenderTarget` _weightmap_rt (`self.WeightmapMID`)))))

(fn `Export RT`
  (`KismetRenderingLibrary.ExportRenderTarget` (`self.Distance Field Cache`) (`self.path`) (`self.Name`)))

(fn `ForceUpdate`
  (bind _brushmanager (`self.BrushManager`))
  (`/Landmass/DistanceFields/Blueprints/JumpFlood_Component2D.JumpFlood` (`/Landmass/Landscape/BlueprintBrushes/LandmassBrushManager.JumpFlood_Component2D` _brushmanager) (`/Landmass/Landscape/BlueprintBrushes/LandmassBrushManager.Depth and Shape RT A` _brushmanager) 50000.0 (`self.Curlparams`) true 0.0))

(fn `Render`
  (params (InIsHeightmap :type Boolean) (InCombinedResult :type "TextureRenderTarget2D Object Reference") (InWeightmapLayerName :type "Name (by ref)"))
  (returns (ReturnValue :type "TextureRenderTarget2D Object Reference"))
  (bind _brushmanager (`self.BrushManager`))
  (set `self.HeightmapRender` InIsHeightmap)
  (`self.Brush Setup` InCombinedResult)
  (if false
    (`KismetSystemLibrary.PrintString` "Material Only Draw"))
  ;[1 1 1] Draw the Material
  (`self.Draw Brush Material`)
  ;[0.1699 0.01189 0.25] Return the result to Landscape
  (return (select `bool` (`self.HeightmapRender`) :`false` (`/Landmass/Landscape/BlueprintBrushes/LandmassBrushManager.Weightmap RT` _brushmanager) :`true` (`/Landmass/Landscape/BlueprintBrushes/LandmassBrushManager.Heightmap RT` _brushmanager))))

(fn `UserConstructionScript`
  (set `self.DistanceFieldIsCached` false))