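; BP_WaterBox is a water box actor that follows the first player's pawn horizontally while keeping its own height.
; Each Tick it copies the pawn's X, Y and yaw, then compares their heights.
; It writes BP_WaterBoxVisible in the MP_Enviroment parameter collection as 0 when the pawn is below the box and 1 otherwise, exposing a visibility switch to materials.
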(event `self.ReceiveTick`
  (params (DeltaSeconds :type "Float (single-precision)"))
  (bind _returnvalue (`GameplayStatics.GetPlayerPawn` 0))
  (bind (_returnvalue_roll _returnvalue_pitch _returnvalue_yaw) (`KismetMathLibrary.BreakRotator` (`self.K2_GetActorRotation` _returnvalue)))
  (bind _z (.z (`self.K2_GetActorLocation`)))
  (`self.K2_SetActorLocation` (`KismetMathLibrary.MakeVector` (.x (`self.K2_GetActorLocation` _returnvalue)) (.y (`self.K2_GetActorLocation` _returnvalue)) _z))
  (`self.K2_SetActorRotation` (`KismetMathLibrary.MakeRotator` 0.0 0.0 _returnvalue_yaw))
  (if (> (- _z (.z (`self.K2_GetActorLocation` _returnvalue))) 0.0)
    (`KismetMaterialLibrary.SetScalarParameterValue` "/Game/Material/Grass/MP_Enviroment.MP_Enviroment" "BP_WaterBoxVisible")
    (else
      (`KismetMaterialLibrary.SetScalarParameterValue` "/Game/Material/Grass/MP_Enviroment.MP_Enviroment" "BP_WaterBoxVisible" 1.0))))

(fn `UserConstructionScript`)