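; Volumetric cloud actor that renders up to three placed cloud volumes, such as EmberGen 3D textures, through a dynamic material on its VolumetricCloud component.
; The construction script creates the material instance, assigns it, then calls UpdateMaterial.
; UpdateMaterial finds BP_Cloud_Placeholder actors and passes each one's inverse world transform, split into four vectors, plus its volume texture and the cloud count to the material.
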(fn `UpdateMaterial`
  (bind _cloud_mid (`self.Cloud MID`))
  (bind _cloud_mid_2 (`self.Cloud MID`))
  (bind _cloud_mid_3 (`self.Cloud MID`))
  (bind _cloud_mid_4 (`self.Cloud MID`))
  (`/Engine/EditorBlueprintResources/StandardMacros.IsValid` _cloud_mid_4
    (:`Is Valid`
      (`MaterialInstanceDynamic.SetScalarParameterValue` _cloud_mid_4 "NbClouds" 0.0)
      (bind _outactors (`GameplayStatics.GetAllActorsOfClass` "/Game/volume_cloud_bp/BP_Cloud_Placeholder.BP_Cloud_Placeholder_C"))
      (bind _output (`|GetArrayItem` _outactors))
      (`/Engine/EditorBlueprintResources/StandardMacros.IsValid` _output
        (:`Is Valid`
          ;[1 1 1] Cloud 1
          (bind (_transformx _transformy _transformz _transformw) (`/Game/volume_cloud_bp/BPF_TransformToVectors.TransformToVectors` (`KismetMathLibrary.InvertTransform` (`SceneComponent.K2_GetComponentToWorld` (`Actor.RootComponent` _output)))))
          (`MaterialInstanceDynamic.SetScalarParameterValue` _cloud_mid_2 "NbClouds" 1.0)
          (`MaterialInstanceDynamic.SetDoubleVectorParameterValue` _cloud_mid_2 "Cloud 1 Transform X" _transformx)
          (`MaterialInstanceDynamic.SetDoubleVectorParameterValue` _cloud_mid_2 "Cloud 1 Transform Y" _transformy)
          (`MaterialInstanceDynamic.SetDoubleVectorParameterValue` _cloud_mid_2 "Cloud 1 Transform Z" _transformz)
          (`MaterialInstanceDynamic.SetDoubleVectorParameterValue` _cloud_mid_2 "Cloud 1 Transform W" _transformw)
          (`MaterialInstanceDynamic.SetTextureParameterValue` _cloud_mid_2 "Cloud 1 3D Texture" (`/Game/volume_cloud_bp/BP_Cloud_Placeholder.Cloud Volume Texture` _output))
          (bind _output_2 (`|GetArrayItem` _outactors 1))
          (`/Engine/EditorBlueprintResources/StandardMacros.IsValid` _output_2
            (:`Is Valid`
              ;[1 1 1] Cloud 2
              (bind (_transformx_2 _transformy_2 _transformz_2 _transformw_2) (`/Game/volume_cloud_bp/BPF_TransformToVectors.TransformToVectors` (`KismetMathLibrary.InvertTransform` (`SceneComponent.K2_GetComponentToWorld` (`Actor.RootComponent` _output_2)))))
              (`MaterialInstanceDynamic.SetScalarParameterValue` _cloud_mid_3 "NbClouds" 2.0)
              (`MaterialInstanceDynamic.SetDoubleVectorParameterValue` _cloud_mid_3 "Cloud 2 Transform X" _transformx_2)
              (`MaterialInstanceDynamic.SetDoubleVectorParameterValue` _cloud_mid_3 "Cloud 2 Transform Y" _transformy_2)
              (`MaterialInstanceDynamic.SetDoubleVectorParameterValue` _cloud_mid_3 "Cloud 2 Transform Z" _transformz_2)
              (`MaterialInstanceDynamic.SetDoubleVectorParameterValue` _cloud_mid_3 "Cloud 2 Transform W" _transformw_2)
              (`MaterialInstanceDynamic.SetTextureParameterValue` _cloud_mid_3 "Cloud 2 3D Texture" (`/Game/volume_cloud_bp/BP_Cloud_Placeholder.Cloud Volume Texture` _output_2))
              (bind _output_3 (`|GetArrayItem` _outactors 2))
              (`/Engine/EditorBlueprintResources/StandardMacros.IsValid` _output_3
                (:`Is Valid`
                  ;[1 1 1] Cloud 3
                  (bind (_transformx_3 _transformy_3 _transformz_3 _transformw_3) (`/Game/volume_cloud_bp/BPF_TransformToVectors.TransformToVectors` (`KismetMathLibrary.InvertTransform` (`SceneComponent.K2_GetComponentToWorld` (`Actor.RootComponent` _output_3)))))
                  (`MaterialInstanceDynamic.SetScalarParameterValue` _cloud_mid "NbClouds" 3.0)
                  (`MaterialInstanceDynamic.SetDoubleVectorParameterValue` _cloud_mid "Cloud 3 Transform X" _transformx_3)
                  (`MaterialInstanceDynamic.SetDoubleVectorParameterValue` _cloud_mid "Cloud 3 Transform Y" _transformy_3)
                  (`MaterialInstanceDynamic.SetDoubleVectorParameterValue` _cloud_mid "Cloud 3 Transform Z" _transformz_3)
                  (`MaterialInstanceDynamic.SetDoubleVectorParameterValue` _cloud_mid "Cloud 3 Transform W" _transformw_3)
                  (`MaterialInstanceDynamic.SetTextureParameterValue` _cloud_mid "Cloud 3 3D Texture" (`/Game/volume_cloud_bp/BP_Cloud_Placeholder.Cloud Volume Texture` _output_3)))))))))))

(fn `UserConstructionScript`
  (bind _cloud__material (`self.Cloud  Material`))
  (bind _cloud_mid (`self.Cloud MID`))
  ;[1 1 1] Create Material Instance Dynamic
  (`/Engine/EditorBlueprintResources/StandardMacros.IsValid` _cloud__material
    (:`Is Valid`
      (`/Landmass/Landscape/BlueprintBrushes/Libraries/LandscapeBrushLibrary.Create and Assign MID` _cloud_mid _cloud__material
        (:`Out`
          (`VolumetricCloudComponent.SetMaterial` (`self.VolumetricCloud`) _cloud_mid)
          (`self.UpdateMaterial`))))))